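; Player controller for click-to-command drone control with a visible mouse cursor and Enhanced Input.
; A click traces under the cursor, selecting an actor tagged Drone or sending the selected drone to the hit location through its AI controller.
; D clears the selection, and debug prints report clicked actors, misses and move results.
; GetActorUnderCursor is a separate Camera-channel trace helper that the event graph does not call.
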(event Input|EnhancedActionEvents|EnhancedInputActionIA_SetDestination_Click
  (params (ActionValue :type Boolean) (ElapsedSeconds :type Float%20%28double-precision%29) (TriggeredSeconds :type Float%20%28double-precision%29) (InputAction :type Input%20Action%20Object%20Reference :default "/Game/TopDown/Input/Actions/IA_SetDestination_Click.IA_SetDestination_Click"))
  (bind _hitresult (Game|Player|GetHitResultUnderCursorbyChannel "TraceTypeQuery1" true))
  (bind (_bblockinghit _binitialoverlap _time _distance _location _impactpoint _normal _impactnormal _physmat _hitactor) (Collision|BreakHitResult _hitresult))
  (:Started
    (if _bblockinghit
      (if (Actor|ActorHasTag _hitactor "Drone")
        (Variables|Default|SetCurrentControledDrone _hitactor)
        (else
          (Development|PrintString (Utilities|GetDisplayName _hitactor))
          (Utilities|IsValid (Variables|Default|GetCurrentControledDrone)
            (:Is%20Valid
              (AI|AIMoveTo (AI|GetAIController (Variables|Default|GetCurrentControledDrone)) _location 0 -1.0 "Default" "Default" true true
                (:OnRequestFailed
                  (Development|PrintString "No work"))
                (:OnMoveFinished
                  (Development|PrintString "Moved")))))))
      (else
        (Development|PrintString "NO HIT" true true "(R=0.000000,G=0.660000,B=1.000000,A=1.000000)" 3.0)))))

(event EventBeginPlay
  (bind _returnvalue (PlayerController|LocalPlayerSubsystems|GetEnhancedInputLocalPlayerSubsystem))
  (Utilities|IsValid _returnvalue
    (:Is%20Valid
      (Input|AddMappingContext _returnvalue "/Game/TopDown/Input/IMC_Default.IMC_Default" 0 "(bIgnoreAllPressedKeysUntilRelease=True,bForceImmediately=False,bNotifyUserSettings=False)")
      (Variables|Default|SetbShowMouseCursor true))))

(event EventTick
  (params (DeltaSeconds :type Float%20%28single-precision%29)))

(event Input|KeyboardEvents|D
  (params (Key :type Key%20Structure :default "None"))
  (:Pressed
    (Variables|Default|SetCurrentControledDrone 0)))

(fn ConstructionScript)

(fn GetActorUnderCursor
  (bind _hitresult (Game|Player|GetHitResultUnderCursorbyChannel "TraceTypeQuery2" true))
  (bind (_bblockinghit _binitialoverlap _time _distance _location _impactpoint _normal _impactnormal _physmat _hitactor) (Collision|BreakHitResult _hitresult))
  (return (== _hitactor "/Game/TopDown/Blueprints/BP_TopDown.BP_TopDown") _location 0))