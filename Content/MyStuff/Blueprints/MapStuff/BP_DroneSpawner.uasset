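; BP_DroneSpawner is a map actor that spawns the player's drones from data stored in GI_CustomGameInstance when play begins.
; It loops over DroneMap and spawns a BP_Drone at one of three Billboard markers, chosen by array index.
; Each drone gets its name, then its HP, shield level and Tow, Scanner and Generator abilities from name-keyed maps in the game instance.
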(event EventBeginPlay
  (bind _asgi_custom_game_instance (Utilities|Casting|CastToGI_CustomGameInstance (Game|GetGameInstance)))
  (bind _output_get (Variables|Default|SetCustom%20Game%20Instance _asgi_custom_game_instance))
  (for (_array_element _array_index) (Variables|/Game/MyStuff/Blueprints/MapStuff/GI_CustomGameInstance.GI_CustomGameInstance_C|GetDroneMap _output_get)
    (bind _returnvalue (Game|SpawnActorfromClass "/Game/MyStuff/Blueprints/BP_Drone.BP_Drone_C" (Utilities|Array|Get(acopy) (Utilities|Array|MakeArray (Transformation|GetWorldTransform (Variables|Default|GetBillboard)) (Transformation|GetWorldTransform (Variables|Default|GetBillboard1)) (Transformation|GetWorldTransform (Variables|Default|GetBillboard2))) _array_index) "AdjustIfPossibleButAlwaysSpawn" "MultiplyWithRoot" 0 0))
    (Variables|/Game/MyStuff/Blueprints/BP_Drone.BP_Drone_C|SetName _returnvalue _array_element)
    (Variables|/Game/MyStuff/Blueprints/BP_Drone.BP_Drone_C|SetHP _returnvalue (.Value (Utilities|Map|Find (Variables|/Game/MyStuff/Blueprints/MapStuff/GI_CustomGameInstance.GI_CustomGameInstance_C|GetHealthMap (Variables|Default|GetCustom%20Game%20Instance)) _array_element)))
    (Variables|/Game/MyStuff/Blueprints/BP_Drone.BP_Drone_C|SetSheildLevel _returnvalue (.Value (Utilities|Map|Find (Variables|/Game/MyStuff/Blueprints/MapStuff/GI_CustomGameInstance.GI_CustomGameInstance_C|GetSheildMap (Variables|Default|GetCustom%20Game%20Instance)) _array_element)))
    (Utilities|Map|Add (Variables|/Game/MyStuff/BPC_Abilities.BPC_Abilities_C|GetAbilityMap (Variables|/Game/MyStuff/Blueprints/BP_Drone.BP_Drone_C|GetBPC_Abilities _returnvalue)) "Tow" (.tow (.Value (Utilities|Map|Find (Variables|/Game/MyStuff/Blueprints/MapStuff/GI_CustomGameInstance.GI_CustomGameInstance_C|GetAbilityMap (Variables|Default|GetCustom%20Game%20Instance)) _array_element))))
    (Utilities|Map|Add (Variables|/Game/MyStuff/BPC_Abilities.BPC_Abilities_C|GetAbilityMap (Variables|/Game/MyStuff/Blueprints/BP_Drone.BP_Drone_C|GetBPC_Abilities _returnvalue)) "Scanner" (.scanner (.Value (Utilities|Map|Find (Variables|/Game/MyStuff/Blueprints/MapStuff/GI_CustomGameInstance.GI_CustomGameInstance_C|GetAbilityMap (Variables|Default|GetCustom%20Game%20Instance)) _array_element))))
    (Utilities|Map|Add (Variables|/Game/MyStuff/BPC_Abilities.BPC_Abilities_C|GetAbilityMap (Variables|/Game/MyStuff/Blueprints/BP_Drone.BP_Drone_C|GetBPC_Abilities _returnvalue)) "Generator" (.generator (.Value (Utilities|Map|Find (Variables|/Game/MyStuff/Blueprints/MapStuff/GI_CustomGameInstance.GI_CustomGameInstance_C|GetAbilityMap (Variables|Default|GetCustom%20Game%20Instance)) _array_element))))))

(event Collision|EventActorBeginOverlap
  (params (OtherActor :type Actor%20Object%20Reference)))

(event EventTick
  (params (DeltaSeconds :type Float%20%28single-precision%29)))

(fn ConstructionScript)