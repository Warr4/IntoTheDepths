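; BP_SpawnRoomBounds is a room bounds actor that tracks which drones are inside it and how many.
; Box overlap events filter for actors tagged Drone, setting or clearing each BP_Drone's CurrentRoomSpawn reference and adjusting the drone count.
; Each change passes the count to the UI held by GI_CustomGameInstance, which is cached on BeginPlay.
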(event OnComponentBeginOverlap(Box)
  (params (OverlappedComponent :type Primitive%20Component%20Object%20Reference) (OtherActor :type Actor%20Object%20Reference) (OtherComp :type Primitive%20Component%20Object%20Reference) (OtherBodyIndex :type Integer) (bFromSweep :type Boolean) (SweepResult :type Hit%20Result%20Structure%20%28by%20ref%29))
  (if (Actor|ActorHasTag OtherActor "Drone")
    (bind _asbp_drone (Utilities|Casting|CastToBP_Drone OtherActor))
    (Variables|/Game/MyStuff/Blueprints/BP_Drone.BP_Drone_C|SetCurrentRoomSpawn _asbp_drone self)
    (bind _output_get (Variables|Default|SetNumber%20of%20drones (+ (Variables|Default|GetNumber%20of%20drones) 1)))
    (Default|Update (Variables|/Game/MyStuff/Blueprints/MapStuff/GI_CustomGameInstance.GI_CustomGameInstance_C|GetUI (Variables|Default|GetGame%20Instance)) _output_get)))

(event OnComponentEndOverlap(Box)
  (params (OverlappedComponent :type Primitive%20Component%20Object%20Reference) (OtherActor :type Actor%20Object%20Reference) (OtherComp :type Primitive%20Component%20Object%20Reference) (OtherBodyIndex :type Integer))
  (if (Actor|ActorHasTag OtherActor "Drone")
    (bind _asbp_drone (Utilities|Casting|CastToBP_Drone OtherActor))
    (Variables|/Game/MyStuff/Blueprints/BP_Drone.BP_Drone_C|SetCurrentRoomSpawn _asbp_drone 0)
    (bind _output_get (Variables|Default|SetNumber%20of%20drones (+ (Variables|Default|GetNumber%20of%20drones) -1)))
    (Default|Update (Variables|/Game/MyStuff/Blueprints/MapStuff/GI_CustomGameInstance.GI_CustomGameInstance_C|GetUI (Variables|Default|GetGame%20Instance)) _output_get)))

(event EventBeginPlay
  (bind _asgi_custom_game_instance (Utilities|Casting|CastToGI_CustomGameInstance (Game|GetGameInstance)))
  (Variables|Default|SetGame%20Instance _asgi_custom_game_instance))

(event Collision|EventActorBeginOverlap
  (params (OtherActor :type Actor%20Object%20Reference)))

(event EventTick
  (params (DeltaSeconds :type Float%20%28single-precision%29)))

(fn ConstructionScript)