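; BP_RoomBounds is a room volume that tracks whether an enemy is inside and shows the result when the room is scanned.
; Box overlaps set or clear a single enemy flag by actor tag, without counting occupants, and entering enemies and drones record it as their current room.
; RoomScanned briefly swaps the cube's outline material to inconclusive, enemy or clear, with inconclusive taking priority, then restores the default clear material.
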(event OnComponentBeginOverlap(Box)
  (params (OverlappedComponent :type Primitive%20Component%20Object%20Reference) (OtherActor :type Actor%20Object%20Reference) (OtherComp :type Primitive%20Component%20Object%20Reference) (OtherBodyIndex :type Integer) (bFromSweep :type Boolean) (SweepResult :type Hit%20Result%20Structure%20%28by%20ref%29))
  (if (Actor|ActorHasTag OtherActor "Enemy")
    (Variables|Default|SetHasEnemy true)
    (bind _asbp_enemy (Utilities|Casting|CastToBP_Enemy OtherActor))
    (Variables|/Game/MyStuff/Blueprints/AIStuff/BP_Enemy.BP_Enemy_C|SetCurrentRoom _asbp_enemy self)
    (elif (Actor|ActorHasTag OtherActor "Drone")
      (bind _asbp_drone (Utilities|Casting|CastToBP_Drone OtherActor))
      (Variables|/Game/MyStuff/Blueprints/BP_Drone.BP_Drone_C|SetCurrentRoom _asbp_drone self))))

(event OnComponentEndOverlap(Box)
  (params (OverlappedComponent :type Primitive%20Component%20Object%20Reference) (OtherActor :type Actor%20Object%20Reference) (OtherComp :type Primitive%20Component%20Object%20Reference) (OtherBodyIndex :type Integer))
  (if (Actor|ActorHasTag OtherActor "Enemy")
    (Variables|Default|SetHasEnemy false)))

(event Custom|RoomScanned
  (bind _cube (Variables|Default|GetCube))
  (if (Variables|Default|GetInconclusive)
    (Rendering|Material|SetMaterial _cube 0 "/Game/MyStuff/Textures/OutlineMat/Outline_Mat_ScanInconclusive.Outline_Mat_ScanInconclusive")
    (elif (Variables|Default|GetHasEnemy)
      (Rendering|Material|SetMaterial _cube 0 "/Game/MyStuff/Textures/OutlineMat/Outline_Mat_Enemy.Outline_Mat_Enemy")
      (else
        (Rendering|Material|SetMaterial _cube 0 "/Game/MyStuff/Textures/OutlineMat/Outline_Mat_ScanClear.Outline_Mat_ScanClear"))))
  (Utilities|FlowControl|Delay 3.0)
  (Rendering|Material|SetMaterial _cube 0 "/Game/MyStuff/Textures/ClearMat.ClearMat"))

(event EventBeginPlay)

(event Collision|EventActorBeginOverlap
  (params (OtherActor :type Actor%20Object%20Reference)))

(event EventTick
  (params (DeltaSeconds :type Float%20%28single-precision%29)))

(fn ConstructionScript)