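; BP_Door is a powered door that opens and closes by snapping its Cube vertically by a fixed offset.
; The Open/Close event works only while Powered and alternates Open and Close through a FlipFlop.
; BeginPlay fires that FlipFlop directly, skipping the power check, when the Open flag is set or otherwise on a random coin flip.
; Tick swaps the Cube's wireframe material to show powered state.
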(event Custom|Open
  (bind _cube (Variables|Default|GetCube))
  (Transformation|SetRelativeLocation _cube (+ (Variables|/Script/Engine.SceneComponent|GetRelativeLocation _cube) "0.000000,0.000000,150.000000") false false))

(event Custom|Close
  (bind _cube (Variables|Default|GetCube))
  (Transformation|SetRelativeLocation _cube (+ (Variables|/Script/Engine.SceneComponent|GetRelativeLocation _cube) "0.000000,0.000000,-150.000000") false false))

(event Custom|Open/Close
  (if (Variables|Default|GetPowered)
    (Utilities|FlowControl|FlipFlop
      (:A
        (CallFunction|Open))
      (:B
        (CallFunction|Close)))))

(event EventBeginPlay
  (if (Variables|Default|GetOpen?)
    (Utilities|FlowControl|FlipFlop :!label _label
      (:A
        (CallFunction|Open))
      (:B
        (CallFunction|Close)))
    (elif (Math|Random|RandomBool)
      (goto _label))))

(event EventTick
  (params (DeltaSeconds :type Float%20%28single-precision%29))
  (bind _cube (Variables|Default|GetCube))
  (if (Variables|Default|GetPowered)
    (Rendering|Material|SetMaterial _cube 0 "/Game/MyStuff/Textures/WireframeMat/Wireframe_Mat.Wireframe_Mat")
    (else
      (Rendering|Material|SetMaterial _cube 0 "/Game/MyStuff/Textures/WireframeMat/Wireframe_Mat_Unpowered.Wireframe_Mat_Unpowered"))))

(fn ConstructionScript)