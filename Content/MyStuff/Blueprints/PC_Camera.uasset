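; Player controller for commanding drones with the mouse from a camera view, with a visible cursor and Enhanced Input mapping.
; Clicks trace under the cursor: live drones become the controlled drone, dead ones the tow victim.
; Other blocking hits send the controlled drone there if it has an AI controller.
; Q clears the selection, and T makes the controlled drone tow the stored victim.
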(event Input|EnhancedActionEvents|EnhancedInputActionIA_SetDestination_Click
  (params (ActionValue :type Boolean) (ElapsedSeconds :type Float%20%28double-precision%29) (TriggeredSeconds :type Float%20%28double-precision%29) (InputAction :type Input%20Action%20Object%20Reference :default "/Game/TopDown/Input/Actions/IA_SetDestination_Click.IA_SetDestination_Click"))
  (bind _hitresult (Game|Player|GetHitResultUnderCursorbyChannel "TraceTypeQuery1" true))
  (bind (_bblockinghit _binitialoverlap _time _distance _location _impactpoint _normal _impactnormal _physmat _hitactor) (Collision|BreakHitResult _hitresult))
  (:Started
    (if _bblockinghit
      (if (Actor|ActorHasTag _hitactor "Drone")
        (bind _asbp_drone (Utilities|Casting|CastToBP_Drone _hitactor))
        (if (Variables|/Game/MyStuff/Blueprints/BP_Drone.BP_Drone_C|GetDead _asbp_drone)
          (Variables|Default|SetTowVictem _asbp_drone)
          (else
            (Variables|Default|SetCurrentControledDrone _asbp_drone)))
        (else
          (Utilities|IsValid (Variables|Default|GetCurrentControledDrone)
            (:Is%20Valid
              (Utilities|IsValid (AI|GetAIController (Variables|Default|GetCurrentControledDrone))
                (:Is%20Valid
                  (Default|Move (Variables|Default|GetCurrentControledDrone) _location))
                (:Is%20Not%20Valid
                  (Development|PrintString "NOPE GOD FUCKING DAMN IT"))))))))))

(event EventBeginPlay
  (bind _returnvalue (PlayerController|LocalPlayerSubsystems|GetEnhancedInputLocalPlayerSubsystem))
  (Utilities|IsValid _returnvalue
    (:Is%20Valid
      (Input|AddMappingContext _returnvalue "/Game/MyStuff/Movement/IMC_Camera.IMC_Camera" 0 "(bIgnoreAllPressedKeysUntilRelease=True,bForceImmediately=False,bNotifyUserSettings=False)")
      (Variables|Default|SetbShowMouseCursor true))))

(event EventTick
  (params (DeltaSeconds :type Float%20%28single-precision%29)))

(event Input|KeyboardEvents|Q
  (params (Key :type Key%20Structure :default "None"))
  (:Pressed
    (Variables|Default|SetCurrentControledDrone 0)))

(event Input|KeyboardEvents|T
  (params (Key :type Key%20Structure :default "None"))
  (bind _currentcontroleddrone (Variables|Default|GetCurrentControledDrone))
  (:Pressed
    (Default|Tow _currentcontroleddrone (Variables|Default|GetTowVictem) _currentcontroleddrone)))

(fn ConstructionScript)

(fn GetActorUnderCursor
  (bind _hitresult (Game|Player|GetHitResultUnderCursorbyChannel "TraceTypeQuery2" true))
  (bind (_bblockinghit _binitialoverlap _time _distance _location _impactpoint _normal _impactnormal _physmat _hitactor) (Collision|BreakHitResult _hitresult))
  (return (== _hitactor "/Game/TopDown/Blueprints/BP_TopDown.BP_TopDown") _location 0))