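; BP_Door is a door that opens and closes by instantly shifting its Cube component up or down along relative Z.
; The Open/Close event toggles it through a FlipFlop, but only while Powered is true.
; On BeginPlay a random bool may trigger that same FlipFlop, so the door randomly starts open or closed.
; Open and Close are also separate events that apply the offset without checking power or current state.
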(event Custom|Open
  (bind _cube (Variables|Default|GetCube))
  (Transformation|SetRelativeLocation _cube (+ (Variables|/Script/Engine.SceneComponent|GetRelativeLocation _cube) "0.000000,0.000000,150.000000") false false))

(event Custom|Close
  (bind _cube (Variables|Default|GetCube))
  (Transformation|SetRelativeLocation _cube (+ (Variables|/Script/Engine.SceneComponent|GetRelativeLocation _cube) "0.000000,0.000000,-150.000000") false false))

(event Custom|Open/Close
  (if (Variables|Default|GetPowered)
    (Utilities|FlowControl|FlipFlop
      (:A
        (CallFunction|Open))
      (:B
        (CallFunction|Close)))))

(event EventBeginPlay
  (if (Math|Random|RandomBool)
    (Utilities|FlowControl|FlipFlop
      (:A
        (CallFunction|Open))
      (:B
        (CallFunction|Close)))))

(fn ConstructionScript)