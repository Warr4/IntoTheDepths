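; BP_Generator is a generator actor that powers a set of doors while a qualified drone is within its sphere.
; On sphere overlap, it checks for the Drone tag, casts to BP_Drone and looks up the Generator entry in the drone's ability map.
; If that ability is true, it sets Powered on every entry in its Doors array, then clears it when the drone leaves the sphere.
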(event OnComponentBeginOverlap(Sphere)
  (params (OverlappedComponent :type Primitive%20Component%20Object%20Reference) (OtherActor :type Actor%20Object%20Reference) (OtherComp :type Primitive%20Component%20Object%20Reference) (OtherBodyIndex :type Integer) (bFromSweep :type Boolean) (SweepResult :type Hit%20Result%20Structure%20%28by%20ref%29))
  (if (Actor|ActorHasTag OtherActor "Drone")
    (bind _asbp_drone (Utilities|Casting|CastToBP_Drone OtherActor))
    (if (.Value (Utilities|Map|Find (Variables|/Game/MyStuff/BPC_Abilities.BPC_Abilities_C|GetAbilityMap (Variables|/Game/MyStuff/Blueprints/BP_Drone.BP_Drone_C|GetBPC_Abilities _asbp_drone)) "Generator"))
      (for _array_element (Variables|Default|GetDoors)
        (Variables|/Game/MyStuff/Blueprints/BP_Door.BP_Door_C|SetPowered _array_element true)))))

(event OnComponentEndOverlap(Sphere)
  (params (OverlappedComponent :type Primitive%20Component%20Object%20Reference) (OtherActor :type Actor%20Object%20Reference) (OtherComp :type Primitive%20Component%20Object%20Reference) (OtherBodyIndex :type Integer))
  (if (Actor|ActorHasTag OtherActor "Drone")
    (bind _asbp_drone (Utilities|Casting|CastToBP_Drone OtherActor))
    (if (.Value (Utilities|Map|Find (Variables|/Game/MyStuff/BPC_Abilities.BPC_Abilities_C|GetAbilityMap (Variables|/Game/MyStuff/Blueprints/BP_Drone.BP_Drone_C|GetBPC_Abilities _asbp_drone)) "Generator"))
      (for _array_element (Variables|Default|GetDoors)
        (Variables|/Game/MyStuff/Blueprints/BP_Door.BP_Door_C|SetPowered _array_element false)))))

(event EventBeginPlay)

(event Collision|EventActorBeginOverlap
  (params (OtherActor :type Actor%20Object%20Reference)))

(event EventTick
  (params (DeltaSeconds :type Float%20%28single-precision%29)))

(fn ConstructionScript)