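; Player controller for top-down drone command: adds the camera input mapping, shows the cursor and binds to every fuel container's drone-in-range event.
; A cursor trace on click routes by actor tag to toggle powered doors, select drones, mark dead drones as tow targets, store interactables or move the selected drone.
; Keys trigger ability-gated tow and cooldown-limited scan, send the drone to a fuel container, or deselect it.
; Selection updates the outline and HUD name colors.
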(event Custom|DoorShinanigans
  (params (InActor :type Actor%20Object%20Reference))
  ;[1 1 1] Abilities
  (bind _asbp_door (Utilities|Casting|CastToBP_Door InActor))
  (if (Variables|/Game/MyStuff/Blueprints/MapStuff/BP_Door.BP_Door_C|GetPowered _asbp_door)
    (Default|Open/Close _asbp_door)))

(event Custom|CustomEvent
  (params (Drone :type Actor%20Object%20Reference))
  ;[1 1 1] Abilities
  (Default|StartFuelDrain (stale Input|KeyboardEvents|R _asbp_fuel_container)))

(event Input|EnhancedActionEvents|EnhancedInputActionIA_SetDestination_Click
  (params (ActionValue :type Boolean) (ElapsedSeconds :type Float%20%28double-precision%29) (TriggeredSeconds :type Float%20%28double-precision%29) (InputAction :type Input%20Action%20Object%20Reference :default "/Game/MyStuff/Movement/Actions/IA_SetDestination_Click.IA_SetDestination_Click"))
  (bind _hitresult (Game|Player|GetHitResultUnderCursorbyChannel "TraceTypeQuery1" true))
  (bind (_bblockinghit _binitialoverlap _time _distance _location _impactpoint _normal _impactnormal _physmat _hitactor) (Collision|BreakHitResult _hitresult))
  ;[1 1 1] Drone Movement
  (:Started
    (if _bblockinghit
      (if (Actor|ActorHasTag _hitactor "Door")
        (CallFunction|DoorShinanigans _hitactor)
        (elif (Actor|ActorHasTag _hitactor "Drone")
          (Rendering|SetVisibility (Variables|/Game/MyStuff/Blueprints/BP_Drone.BP_Drone_C|GetSelectionOutline (Variables|Default|GetCurrentControledDrone)) false false)
          (bind _asbp_drone (Utilities|Casting|CastToBP_Drone _hitactor))
          (if (Variables|/Game/MyStuff/Blueprints/BP_Drone.BP_Drone_C|GetDead _asbp_drone)
            (Variables|Default|SetTowVictem _asbp_drone)
            (else
              (Rendering|SetVisibility (Variables|/Game/MyStuff/Blueprints/BP_Drone.BP_Drone_C|GetSelectionOutline _asbp_drone) true false)
              (bind _output_get (Variables|Default|SetCurrentControledDrone _asbp_drone))
              (for _array_element (Variables|/Script/Engine.Actor|GetTags _output_get)
                (for _array_element_2 (Variables|/Game/MyStuff/Blueprints/GI_CustomGameInstance.GI_CustomGameInstance_C|GetHP%20Widgets (Variables|Default|GetGame%20Instance))
                  (if (Utilities|Enum|Equal(Enum) (Variables|/Script/UMG.TextBlock|GetText (Variables|/Game/MyStuff/UI/WBP_DroneHP.WBP_DroneHP_C|GetDronename _array_element_2)) (Utilities|Text|ToText(Name) _array_element))
                    (Appearance|SetColorandOpacity (Variables|/Game/MyStuff/UI/WBP_DroneHP.WBP_DroneHP_C|GetDronename _array_element_2) (Utilities|Struct|MakeSlateColor "(R=1.000000,G=1.000000,B=1.000000,A=1.000000)" "UseColor_Specified") :!class /Script/UMG.TextBlock)
                    (else
                      (Appearance|SetColorandOpacity (Variables|/Game/MyStuff/UI/WBP_DroneHP.WBP_DroneHP_C|GetDronename _array_element_2) (Utilities|Struct|MakeSlateColor "(R=0.000000,G=1.000000,B=1.000000,A=1.000000)" "UseColor_Specified") :!class /Script/UMG.TextBlock)))))))
          (elif (Actor|ActorHasTag _hitactor "Interactable")
            (Variables|Default|SetInteractableObject _hitactor)
            (else
              (Utilities|IsValid (Variables|Default|GetCurrentControledDrone)
                (:Is%20Valid
                  (Utilities|IsValid (AI|GetAIController (Variables|Default|GetCurrentControledDrone))
                    (:Is%20Valid
                      (Default|Move (Variables|Default|GetCurrentControledDrone) _location))))))))))))

(event EventBeginPlay
  (bind _returnvalue (PlayerController|LocalPlayerSubsystems|GetEnhancedInputLocalPlayerSubsystem))
  ;[1 1 1] Event Begin Play Stuff
  (Utilities|FlowControl|Sequence
    (:then_0
      (Utilities|IsValid _returnvalue
        (:Is%20Valid
          (Input|AddMappingContext _returnvalue "/Game/MyStuff/Movement/IMC_Camera.IMC_Camera" 0 "(bIgnoreAllPressedKeysUntilRelease=True,bForceImmediately=False,bNotifyUserSettings=False)")
          (Variables|Default|SetbShowMouseCursor true)
          (bind _asgi_custom_game_instance (Utilities|Casting|CastToGI_CustomGameInstance (Game|GetGameInstance)))
          (Variables|Default|SetGame%20Instance _asgi_custom_game_instance))))
    (:then_1
      (bind _outactors (Actor|GetAllActorsOfClass "/Game/MyStuff/Blueprints/MapStuff/BP_FuelContainer.BP_FuelContainer_C"))
      (for _array_element _outactors
        (EventDispatchers|BindEventtoOnDroneinRange _array_element (EventDispatchers|CreateEvent :!event Custom|CustomEvent))))))

(event Input|KeyboardEvents|E
  (params (Key :type Key%20Structure :default "None"))
  (bind _currentcontroleddrone (Variables|Default|GetCurrentControledDrone))
  ;[1 1 1] Abilities
  (:Pressed
    (Utilities|FlowControl|DoOnce false :!label _label
      (:Completed
        (if (.Value (Utilities|Map|Find (Variables|/Game/MyStuff/BPC_Abilities.BPC_Abilities_C|GetAbilityMap (Variables|/Game/MyStuff/Blueprints/BP_Drone.BP_Drone_C|GetBPC_Abilities _currentcontroleddrone)) "Scanner"))
          (Default|Scan _currentcontroleddrone)
          (Utilities|FlowControl|Delay 1e+01)
          (goto _label Reset)
          (else
            (goto _label Reset)))))))

(event Input|KeyboardEvents|Q
  (params (Key :type Key%20Structure :default "None"))
  ;[1 1 1] Abilities
  (:Pressed
    (Variables|Default|SetCurrentControledDrone 0)))

(event Input|KeyboardEvents|T
  (params (Key :type Key%20Structure :default "None"))
  (bind _currentcontroleddrone (Variables|Default|GetCurrentControledDrone))
  ;[1 1 1] Abilities
  (:Pressed
    (if (.Value (Utilities|Map|Find (Variables|/Game/MyStuff/BPC_Abilities.BPC_Abilities_C|GetAbilityMap (Variables|/Game/MyStuff/Blueprints/BP_Drone.BP_Drone_C|GetBPC_Abilities _currentcontroleddrone)) "Tow"))
      (Default|Tow _currentcontroleddrone (Variables|Default|GetTowVictem) _currentcontroleddrone))))

(event Input|KeyboardEvents|R
  (params (Key :type Key%20Structure :default "None"))
  ;[1 1 1] Abilities
  (:Pressed
    (bind _asbp_fuel_container (Utilities|Casting|CastToBP_FuelContainer (Variables|Default|GetInteractableObject)))
    (Default|Move (Variables|Default|GetCurrentControledDrone) (Transformation|GetWorldLocation (Variables|/Game/MyStuff/Blueprints/MapStuff/BP_FuelContainer.BP_FuelContainer_C|GetBillboard _asbp_fuel_container)))))

(fn ConstructionScript)

(fn GetActorUnderCursor
  (bind _hitresult (Game|Player|GetHitResultUnderCursorbyChannel "TraceTypeQuery2" true))
  (bind (_bblockinghit _binitialoverlap _time _distance _location _impactpoint _normal _impactnormal _physmat _hitactor) (Collision|BreakHitResult _hitresult))
  (return (== _hitactor "/Game/TopDown/Blueprints/BP_TopDown.BP_TopDown") _location 0))