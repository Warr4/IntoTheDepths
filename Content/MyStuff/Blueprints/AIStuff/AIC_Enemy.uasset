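; Enemy AI controller that wanders the navmesh and chases living pawns tagged "Drone".
; A looping timer moves it to random nearby points until PawnSensing sees a drone.
; A DoOnce-gated sighting starts looping Attack moves toward the drone and a chase countdown.
; Arrival stops the attack timer, failure or timeout also restarts wandering, and each outcome reopens the gate.
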(event OnSeePawn(PawnSensing)
  (params (Pawn :type Pawn%20Object%20Reference))
  (if (Actor|ActorHasTag Pawn "Drone")
    (if (not (Actor|ActorHasTag Pawn "Dead"))
      (Variables|Default|SetDrone Pawn)
      (Utilities|FlowControl|DoOnce false
        (:Completed
          (bind _returnvalue (Utilities|Time|SetTimerbyFunctionName 0 "Attack" 0.1 true))
          (Variables|Default|SetAttack%20Timer _returnvalue)
          (bind _returnvalue_2 (Utilities|Time|SetTimerbyFunctionName 0 "ChaseTimer" 0.1 true))
          (Variables|Default|SetChaseTimerHandle _returnvalue_2))))))

(event Custom|Attack
  (bind _drone (Variables|Default|GetDrone))
  (bind _attack_timer (Variables|Default|GetAttack%20Timer))
  (Utilities|IsValid _drone
    (:Is%20Valid
      (Utilities|Time|ClearandInvalidateTimerbyHandle (Variables|Default|GetWander%20Timer))
      (AI|AIMoveTo 0 (Transformation|GetActorLocation _drone) 0 15.0 false
        (:OnSuccess
          (Utilities|Time|ClearandInvalidateTimerbyHandle _attack_timer)
          (Utilities|FlowControl|Delay 1.0)
          (CallFunction|OpenDoOnce))
        (:OnFail
          (CallFunction|Wander)
          (Utilities|Time|ClearandInvalidateTimerbyHandle _attack_timer)
          (CallFunction|OpenDoOnce))))))

(event Custom|Wander
  (bind _returnvalue (Utilities|Time|SetTimerbyEvent (delegate Custom|WanderTo) 3.0 true))
  (Variables|Default|SetWander%20Timer _returnvalue))

(event Custom|WanderTo
  (bind _returnvalue (Pawn|GetControlledPawn))
  (bind _randomlocation (Class|NavigationSystemV1|GetRandomLocationinNavigableRadius (Transformation|GetActorLocation _returnvalue) 5e+02 0 0))
  (AI|AIMoveTo _returnvalue _randomlocation 0 5.0 false))

(event Custom|ChaseTimer
  (bind _output_get (Variables|Default|SetTime (- (Variables|Default|GetTime) 0.1)))
  (if (<= _output_get 0.0)
    (Utilities|Time|ClearandInvalidateTimerbyHandle (Variables|Default|GetAttack%20Timer))
    (Utilities|Time|ClearandInvalidateTimerbyHandle (Variables|Default|GetChaseTimerHandle))
    (CallFunction|Wander)
    (Utilities|FlowControl|Delay 0.5)
    (CallFunction|OpenDoOnce)))

(event Custom|OpenDoOnce
  (Utilities|FlowControl|DoOnce false) ; enters at Reset
)

(event EventBeginPlay
  (CallFunction|Wander))

(event EventTick
  (params (DeltaSeconds :type Float%20%28single-precision%29)))

(fn ConstructionScript)