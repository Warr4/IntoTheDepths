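; Enemy actor that spawns in a room and damages nearby actors tagged "Drone".
; On BeginPlay it teleports to a random BP_RoomBounds actor, or to SpawnRoom on TestMap.
; Each tick it runs a debug-drawn multi-sphere trace around itself, feeding hits through a DoOnce.
; A Drone hit takes damage and re-arms the gate after a short delay, while other hits re-arm it immediately.
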(event OnComponentBeginOverlap(Box)
  (params (OverlappedComponent :type Primitive%20Component%20Object%20Reference) (OtherActor :type Actor%20Object%20Reference) (OtherComp :type Primitive%20Component%20Object%20Reference) (OtherBodyIndex :type Integer) (bFromSweep :type Boolean) (SweepResult :type Hit%20Result%20Structure%20%28by%20ref%29)))

(event Custom|ResetDoOnce
  (Utilities|FlowControl|DoOnce false) ; enters at Reset
)

(event EventBeginPlay
  (bind _returnvalue (Game|GetCurrentLevelName true))
  (if (not (Utilities|Enum|Equal(Enum) _returnvalue "TestMap"))
    (bind _outactors (Actor|GetAllActorsOfClass "/Game/MyStuff/Blueprints/MapStuff/BP_RoomBounds.BP_RoomBounds_C"))
    (Transformation|SetActorLocation (Transformation|GetActorLocation (.OutItem (Utilities|Array|Random _outactors))) false true)
    (else
      (Transformation|SetActorLocation (Transformation|GetActorLocation (Variables|Default|GetSpawnRoom)) false true))))

(event Collision|EventActorBeginOverlap
  (params (OtherActor :type Actor%20Object%20Reference)))

(event EventTick
  (params (DeltaSeconds :type Float%20%28single-precision%29))
  (bind _returnvalue (Transformation|GetActorLocation))
  (bind _outhits (Collision|MultiSphereTraceByChannel _returnvalue _returnvalue 1.5e+02 "TraceTypeQuery1" false 0 "ForOneFrame"))
  (for _array_element _outhits
    (Utilities|FlowControl|DoOnce false
      (:Completed
        (if (Actor|ActorHasTag (.HitActor (Collision|BreakHitResult _array_element)) "Drone")
          (Game|Damage|ApplyDamage (.HitActor (Collision|BreakHitResult _array_element)) 1.0 0 0)
          (Utilities|FlowControl|Delay 2.0)
          (CallFunction|ResetDoOnce)
          (else
            (CallFunction|ResetDoOnce)))))))

(fn ConstructionScript)